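; Interactive console actor that reacts when the player selects or deselects it.
; Selection switches the Screen mesh to its lit material and, only on first activation, plays an up beep and sets the Active flag.
; Deselection restores the off material, plays a down beep and clears Active.
; Both events also print on-screen debug messages.
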(event EventTick
  (params (DeltaSeconds :type Float%20%28single-precision%29))
  (|CallParentFunction DeltaSeconds))

(event EventDeSelected
  ;[1 1 1] When Deselected By the Player
  (Development|PrintString "I'm deselected" true true "(R=1.000000,G=0.941159,B=0.000000,A=1.000000)")
  (Rendering|Material|SetMaterial (Variables|Default|GetScreen) 0 "/Game/Materials/M_Console_Screen_Off.M_Console_Screen_Off")
  (Audio|PlaySound2D "/Game/Sounds/SQ_DownBeep.SQ_DownBeep" 1.0 1.0 0.0 0 0)
  (Variables|Default|SetActive false))

(event EventSelected
  ;[1 1 1] When Selected By the Player
  (Development|PrintString "I'm being selected!" true true "(R=1.000000,G=0.988851,B=0.000000,A=1.000000)")
  (Rendering|Material|SetMaterial (Variables|Default|GetScreen) 0 "/Game/Materials/M_Console_Screen_On.M_Console_Screen_On")
  (if (not (Variables|Default|GetActive))
    (Audio|PlaySound2D "/Game/Sounds/SQ_UpBeep.SQ_UpBeep" 1.0 1.0 0.0 0 0)
    (Variables|Default|SetActive true)))

(event EventBeginPlay
  (|CallParentFunction))

(event Collision|EventActorBeginOverlap
  (params (OtherActor :type Actor%20Object%20Reference))
  (|CallParentFunction OtherActor))

(fn ConstructionScript
  (|CallParentFunction))